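; Trap-style shooter actor that fires Arrow actors when the player character crosses its line of sight.
; Each Tick, a sphere trace runs forward from ArrowSource and calls ShootArrow when it hits the player.
; ShootArrow spawns an arrow at ArrowSource and plays a sound at world origin, with a DoOnce and Delay acting as cooldown.
; A looping timer for ShootArrow is present but never runs.
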(event Custom|ShootArrow
  (Utilities|FlowControl|DoOnce false :!label _label
    (:Completed
      (Game|SpawnActorfromClass "/Game/Blueprints/Arrow.Arrow_C" (Transformation|GetWorldTransform (Variables|Default|GetArrowSource)) "Undefined" 0 0)
      (Audio|PlaySoundatLocation "/Game/Sounds/Arrow_SFX.Arrow_SFX" "0, 0, 0" "0, 0, 0" 1.0 1.0 0.0 0 0 0 0)
      (Utilities|FlowControl|Delay 1.5)
      (goto _label Reset))))

(event EventTick
  (params (DeltaSeconds :type Float%20%28single-precision%29))
  (bind _arrowsource (Variables|Default|GetArrowSource))
  (bind _returnvalue (Transformation|GetWorldLocation _arrowsource))
  (bind _outhit (Collision|SphereTraceByChannel _returnvalue (+ _returnvalue (* (Math|Vector|GetForwardVector (Transformation|GetWorldRotation _arrowsource)) "3000.000000,3000.000000,3000.000000")) 1e+01 "TraceTypeQuery2" false 0 "None"))
  (if (== (.hitactor _outhit) (Game|GetPlayerCharacter 0))
    (CallFunction|ShootArrow)))

(fn ConstructionScript)